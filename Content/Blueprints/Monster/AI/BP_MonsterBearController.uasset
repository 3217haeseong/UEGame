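; BP_MonsterBearController is the AI controller for the bear monster.
; On possess, it sets up the BB_MonsterBear blackboard and seeds it with the patrol wait time and the pawn's current location as its origin.
; It then runs the BT_MonsterBear behavior tree, leaving all further decisions to that tree.
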(event EventPossess
  (params (PossessedPawn :type Pawn%20Object%20Reference))
  (Utilities|FlowControl|Sequence
    (:then_0
      (Class|AIController|UseBlackboard "/Game/Blueprints/Monster/AI/BB_MonsterBear.BB_MonsterBear")
      (AI|Components|Blackboard|SetValueasFloat (Variables|Default|GetBlackboard) (Variables|Default|GetPatrolWaitTimeKey) (Variables|Default|GetPatrolWaitTime))
      (AI|Components|Blackboard|SetValueasVector (Variables|Default|GetBlackboard) (Variables|Default|GetOriginLocationKey) (Transformation|GetActorLocation PossessedPawn)))
    (:then_1
      (AI|RunBehaviorTree "/Game/Blueprints/Monster/AI/BT_MonsterBear.BT_MonsterBear"))))

(fn ConstructionScript)