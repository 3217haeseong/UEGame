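; BP_DamageReceiver is a component that tracks an actor's health and handles incoming damage, with a brief invulnerability window after each hit.
; Health starts at its maximum on BeginPlay, and damage is applied only while Vulnerable, which a timer restores after InvulnerableTime.
; Each accepted hit broadcasts a health-changed event, and health reaching zero is clamped and also fires a death event.
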(event Custom|OnDamageReceived
  (params (Damage :type Float%20%28double-precision%29))
  (if (Variables|Default|Getvulnerable)
    (Variables|Default|Setvulnerable false)
    (Utilities|Time|SetTimerbyEvent (delegate Custom|ReturnToVulnerable) (Variables|Default|GetInvulnerableTime)) ; 일정시간 무적 상태를 만드는 타이머
    (Variables|Default|SetHealthPower (- (Variables|Default|GetHealthPower) Damage))
    (if (<= (Variables|Default|GetHealthPower) 0.0)
      (Variables|Default|SetHealthPower 0.0)
      (Default|CallOnDead)
      (Default|CallOnHealthPowerChanged (Variables|Default|GetHealthPower) (Variables|Default|GetMaxHealthPower))
      (else
        (Default|CallOnHealthPowerChanged (Variables|Default|GetHealthPower) (Variables|Default|GetMaxHealthPower))))))

(event Custom|ReturnToVulnerable
  (Variables|Default|Setvulnerable true))

(event EventBeginPlay
  (Variables|Default|SetHealthPower (Variables|Default|GetMaxHealthPower)))